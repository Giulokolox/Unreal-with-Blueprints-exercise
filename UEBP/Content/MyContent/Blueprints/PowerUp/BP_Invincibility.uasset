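; BP_Invincibility is a power-up pickup that toggles the player's Invincible flag for a timed period.
; Overlapping its Box with a BP_Player sets Invincible to false, then back to true after a five-second Delay, so the flag reads inverted relative to its name.
; The PickUp event separately triggers the player's invincibility pickup message, destroys the Niagara effect and calls KillYourself.
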(event OnComponentBeginOverlap(Box)
  (params (OverlappedComponent :type Primitive%20Component%20Object%20Reference) (OtherActor :type Actor%20Object%20Reference) (OtherComp :type Primitive%20Component%20Object%20Reference) (OtherBodyIndex :type Integer) (bFromSweep :type Boolean) (SweepResult :type Hit%20Result%20Structure%20%28by%20ref%29))
  ;[1 1 1] Invincible method
  (bind _asbp_player (Utilities|Casting|CastToBP_Player OtherActor))
  (Variables|/Game/MyContent/Blueprints/Player/BP_Player.BP_Player_C|SetInvincible _asbp_player false)
  (Utilities|FlowControl|Delay 5.0)
  (Variables|/Game/MyContent/Blueprints/Player/BP_Player.BP_Player_C|SetInvincible _asbp_player true))

(event EventPickUp
  ;[1 1 1] event pick up
  (Class|IPickUp|PickUpInvincibility(Message) (Game|GetPlayerCharacter 0))
  (Components|DestroyComponent (Variables|Default|GetNiagara))
  (CallFunction|KillYourself))

(fn ConstructionScript
  (|CallParentFunction))