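; BP_PickUpBase is a base pickup Blueprint whose Box overlap calls PickUp when the other actor carries the Player tag.
; PickUp is empty here, so the base defines no pickup effect of its own.
; KillYourself hides the StaticMesh and disables Box and mesh collision rather than destroying the actor.
; Reset performs the same hide and disable steps, so it does not restore the pickup.
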(event OnComponentBeginOverlap(Box)
  (params (OverlappedComponent :type Primitive%20Component%20Object%20Reference) (OtherActor :type Actor%20Object%20Reference) (OtherComp :type Primitive%20Component%20Object%20Reference) (OtherBodyIndex :type Integer) (bFromSweep :type Boolean) (SweepResult :type Hit%20Result%20Structure%20%28by%20ref%29))
  (if (Actor|ActorHasTag OtherActor "Player")
    (CallFunction|PickUp)))

(event Custom|PickUp)

(event Custom|KillYourself
  (Development|SetHiddeninGame (Variables|Default|GetStaticMesh) true false)
  (Collision|SetCollisionEnabled (Variables|Default|GetBox) "NoCollision"))

(event Custom|Reset
  (Development|SetHiddeninGame (Variables|Default|GetStaticMesh) true false)
  (Collision|SetCollisionEnabled (Variables|Default|GetBox) "NoCollision"))

(fn ConstructionScript)