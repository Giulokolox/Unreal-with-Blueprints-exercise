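; BP_DeathZone is a trigger volume that ends play when BP_Player enters it.
; On box overlap it adds a WBP_Death widget to the viewport, shows the mouse cursor, pauses the game and destroys itself.
; The construction script sets the box's world transform from the Height and Size variables, controlling its Z position and horizontal scale.
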(event OnComponentBeginOverlap(Box)
  (params (OverlappedComponent :type Primitive%20Component%20Object%20Reference) (OtherActor :type Actor%20Object%20Reference) (OtherComp :type Primitive%20Component%20Object%20Reference) (OtherBodyIndex :type Integer) (bFromSweep :type Boolean) (SweepResult :type Hit%20Result%20Structure%20%28by%20ref%29))
  (Utilities|Casting|CastToBP_Player OtherActor)
  (bind _returnvalue (UserInterface|CreateWidget "/Game/MyContent/Blueprints/Ui/WBP_Death.WBP_Death_C" (Game|GetPlayerController 0)))
  (UserInterface|Viewport|AddtoViewport _returnvalue 0)
  (Variables|/Script/Engine.PlayerController|SetbShowMouseCursor (Game|GetPlayerController 0) true)
  (Game|SetGamePaused true)
  (Actor|DestroyActor))

(fn ConstructionScript
  (bind _size (Variables|Default|GetSize))
  (Transformation|SetWorldTransform (Variables|Default|GetBox) (Math|Transform|MakeTransform (Math|Vector|MakeVector 0.0 0.0 (Variables|Default|GetHeight)) "0, 0, 0" (Math|Vector|MakeVector _size _size 1.0)) false false))