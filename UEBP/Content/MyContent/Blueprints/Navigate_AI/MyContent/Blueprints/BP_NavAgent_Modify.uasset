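; BP_NavAgent_Modify is a wandering enemy NPC that damages the player on contact and can be killed for a power-up.
; MoveNPC loops AI Move To toward random reachable points near random TargetList actors, pausing briefly between moves.
; Capsule overlap with BP_Player applies delayed damage.
; Box overlap increments the player's Enemies kill count, destroys the agent and spawns BP_Invincibility at its transform.
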(event OnComponentBeginOverlap(Box)
  (params (OverlappedComponent :type Primitive%20Component%20Object%20Reference) (OtherActor :type Actor%20Object%20Reference) (OtherComp :type Primitive%20Component%20Object%20Reference) (OtherBodyIndex :type Integer) (bFromSweep :type Boolean) (SweepResult :type Hit%20Result%20Structure%20%28by%20ref%29))
  ;[1 1 1] Kill count with spawn power up
  (bind _asbp_player (Utilities|Casting|CastToBP_Player OtherActor))
  (Variables|/Game/MyContent/Blueprints/Player/BP_Player.BP_Player_C|SetEnemies _asbp_player (+ (Variables|/Game/MyContent/Blueprints/Player/BP_Player.BP_Player_C|GetEnemies _asbp_player) 1))
  (Utilities|FlowControl|Delay 0.2)
  (Components|DestroyComponent (Variables|Character|GetMesh))
  (Actor|DestroyActor)
  (Game|SpawnActorfromClass "/Game/MyContent/Blueprints/PowerUp/BP_Invincibility.BP_Invincibility_C" (Transformation|GetActorTransform) "Undefined" 0 0)
  (Utilities|FlowControl|Delay 1.0))

(event OnComponentBeginOverlap(Capsule)
  (params (OverlappedComponent :type Primitive%20Component%20Object%20Reference) (OtherActor :type Actor%20Object%20Reference) (OtherComp :type Primitive%20Component%20Object%20Reference) (OtherBodyIndex :type Integer) (bFromSweep :type Boolean) (SweepResult :type Hit%20Result%20Structure%20%28by%20ref%29))
  ;[1 1 1] Damage
  (bind _asbp_player (Utilities|Casting|CastToBP_Player OtherActor))
  (Utilities|FlowControl|Delay 0.7)
  (Game|Damage|ApplyDamage _asbp_player 3e+01 0 0))

(event Custom|MoveNPC
  (bind _targetlist (Variables|Default|GetTargetList))
  (bind _output_get (Variables|Default|SetCurrentTarget (Utilities|Array|Get(acopy) _targetlist (Math|Random|RandomIntegerinRange 0 (Utilities|Array|LastIndex _targetlist)))))
  (Utilities|IsValid _output_get
    (:Is%20Valid
      (bind _output_get_2 (Variables|Default|SetRandom%20Location (.RandomLocation (AI|Navigation|GetRandomReachablePointinRadius (Transformation|GetActorLocation (Variables|Default|GetCurrentTarget)) 1e+02 0 0))))
      (AI|AIMoveTo self _output_get_2 0 5.0 false
        (:OnSuccess
          (Utilities|FlowControl|Delay 2.0)
          (CallFunction|MoveNPC))
        (:OnFail
          (Utilities|FlowControl|Delay 0.1)
          (CallFunction|MoveNPC))))))

(event EventBeginPlay
  (CallFunction|MoveNPC))

(fn ConstructionScript)