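; BP_Key is a pickup that grants the player a key, likely for opening doors.
; When BP_Player overlaps the Radius component, it adds its KeyID to the player's KeyRing without duplicates and destroys itself.
; The construction script applies the key's material to the cube and sets the point light color, so each placed key can have its own look.
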(event OnComponentBeginOverlap(Radius)
  (params (OverlappedComponent :type Primitive%20Component%20Object%20Reference) (OtherActor :type Actor%20Object%20Reference) (OtherComp :type Primitive%20Component%20Object%20Reference) (OtherBodyIndex :type Integer) (bFromSweep :type Boolean) (SweepResult :type Hit%20Result%20Structure%20%28by%20ref%29))
  (bind _asbp_player (Utilities|Casting|CastToBP_Player OtherActor))
  (Utilities|Array|AddUnique (Variables|/Game/MyContent/Blueprints/Player/BP_Player.BP_Player_C|GetKeyRing _asbp_player) (Variables|Default|GetKeyID))
  (Actor|DestroyActor))

(fn ConstructionScript
  (Rendering|Material|SetMaterial (Variables|Default|GetCube) 0 (Variables|Default|GetKeyMat))
  (Rendering|Components|Light|SetLightColor (Variables|Default|GetPointLight) (Variables|Default|GetLifgtColor) true))