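; Sliding door Blueprint that opens when the player enters its Radius trigger and closes when they leave.
; If Locked is set, it opens only when BP_Player holds at least five coins, which it checks but does not deduct.
; The Position timeline lerps the Cube sideways along local Y from its BeginPlay location, and reverses to close.
; A DoorOpen flag ensures closing only follows an actual opening.
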(event OnComponentBeginOverlap(Radius)
  (params (OverlappedComponent :type Primitive%20Component%20Object%20Reference) (OtherActor :type Actor%20Object%20Reference) (OtherComp :type Primitive%20Component%20Object%20Reference) (OtherBodyIndex :type Integer) (bFromSweep :type Boolean) (SweepResult :type Hit%20Result%20Structure%20%28by%20ref%29))
  (bind _asbp_player (Utilities|Casting|CastToBP_Player OtherActor))
  (if (Variables|Default|GetLocked?)
    (if (>= (Variables|/Game/MyContent/Blueprints/Player/BP_Player.BP_Player_C|GetCoins _asbp_player) 5)
      (CallFunction|OpenDoor)
      (Variables|Default|SetDoorOpen true))
    (else
      (CallFunction|OpenDoor)
      (Variables|Default|SetDoorOpen true))))

(event OnComponentEndOverlap(Radius)
  (params (OverlappedComponent :type Primitive%20Component%20Object%20Reference) (OtherActor :type Actor%20Object%20Reference) (OtherComp :type Primitive%20Component%20Object%20Reference) (OtherBodyIndex :type Integer))
  (Utilities|Casting|CastToBP_Player OtherActor)
  (if (Variables|Default|GetDoorOpen)
    (CallFunction|CloseDoor)
    (Variables|Default|SetDoorOpen false)))

(event Custom|OpenDoor
  (bind _startposition (Variables|Default|GetStartPosition))
  (bind _speed (Timeline|Position Play)
    (:Update
      (Transformation|SetRelativeLocation (Variables|Default|GetCube) (Math|Vector|Lerp(Vector) _startposition (- _startposition "0,-180.000000,0.000000") _speed) false false))))

(event Custom|CloseDoor
  (bind _startposition (Variables|Default|GetStartPosition))
  (bind _speed (Timeline|Position Reverse)
    (:Update
      (Transformation|SetRelativeLocation (Variables|Default|GetCube) (Math|Vector|Lerp(Vector) _startposition (- _startposition "0,-180.000000,0.000000") _speed) false false))))

(event EventBeginPlay
  (Variables|Default|SetStartPosition (Variables|/Script/Engine.SceneComponent|GetRelativeLocation (Variables|Default|GetCube))))

(fn ConstructionScript)