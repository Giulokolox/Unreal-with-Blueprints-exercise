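; BP_EnemyCtrl is the AI controller for BP_Enemy, driving patrol and player detection through the BT_Enemy behavior tree.
; On BeginPlay it runs the tree, caches the pawn and seeds the Blackboard with its patrol path's looping and wait settings plus a starting direction.
; AI Perception updates for the player pawn write the sensed state to CanSeePlayer, but only when the Aggressive flag is set.
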(event OnTargetPerceptionUpdated(AIPerception)
  (params (Actor :type Actor%20Object%20Reference) (Stimulus :type AI%20Stimulus%20Structure))
  (if (== Actor (Game|Player|GetPlayerPawn 0))
    (if (Variables|Default|GetAggressive)
      (AI|Components|Blackboard|SetValueasBool (AI|GetBlackboard 0) (Utilities|Name|MakeLiteralName "CanSeePlayer") (.bSuccessfullySensed (Utilities|Struct|BreakAIStimulus Stimulus))))))

(event EventBeginPlay
  (bind _returnvalue (AI|GetBlackboard 0))
  (AI|RunBehaviorTree "/Game/MyContent/Blueprints/AI/BT_Enemy.BT_Enemy")
  (bind _asbp_enemy (Utilities|Casting|CastToBP_Enemy (Pawn|GetControlledPawn)))
  (bind _output_get (Variables|Default|SetMyPawn _asbp_enemy))
  (AI|Components|Blackboard|SetValueasBool (AI|GetBlackboard 0) (Utilities|Name|MakeLiteralName "PathLooping") (Variables|/Game/MyContent/Blueprints/AI/PatrolPath.PatrolPath_C|GetIsLooping (Variables|/Game/MyContent/Blueprints/AI/BP_Enemy.BP_Enemy_C|GetPatrolPath _output_get)))
  (Class|BlackboardComponent|SetValueasInt _returnvalue (Utilities|Name|MakeLiteralName "Direction") 1)
  (AI|Components|Blackboard|SetValueasFloat _returnvalue (Utilities|Name|MakeLiteralName "WaitTime") (Variables|/Game/MyContent/Blueprints/AI/PatrolPath.PatrolPath_C|GetWaitTime (Variables|/Game/MyContent/Blueprints/AI/BP_Enemy.BP_Enemy_C|GetPatrolPath (Variables|Default|GetMyPawn)))))

(fn ConstructionScript)