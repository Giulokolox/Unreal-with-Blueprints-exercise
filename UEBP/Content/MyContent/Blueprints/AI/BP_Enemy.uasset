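; BP_Enemy is an enemy actor that damages the player on contact and can be killed by overlap, dropping a health pickup.
; A player overlapping the Box increments the player's Enemies counter, then after a short delay destroys the enemy and spawns BP_Health at its transform.
; A player overlapping the Capsule instead receives fixed damage through ApplyDamage.
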(event OnComponentBeginOverlap(Box)
  (params (OverlappedComponent :type Primitive%20Component%20Object%20Reference) (OtherActor :type Actor%20Object%20Reference) (OtherComp :type Primitive%20Component%20Object%20Reference) (OtherBodyIndex :type Integer) (bFromSweep :type Boolean) (SweepResult :type Hit%20Result%20Structure%20%28by%20ref%29))
  ;[1 1 1] Kill count with spawn power up
  (bind _asbp_player (Utilities|Casting|CastToBP_Player OtherActor))
  (Variables|/Game/MyContent/Blueprints/Player/BP_Player.BP_Player_C|SetEnemies _asbp_player (+ (Variables|/Game/MyContent/Blueprints/Player/BP_Player.BP_Player_C|GetEnemies _asbp_player) 1))
  (Utilities|FlowControl|Delay 0.2)
  (Components|DestroyComponent (Variables|Character|GetMesh))
  (Actor|DestroyActor)
  (Game|SpawnActorfromClass "/Game/MyContent/Blueprints/PowerUp/BP_Health.BP_Health_C" (Transformation|GetActorTransform) "Undefined" 0 0)
  (Utilities|FlowControl|Delay 1.0))

(event OnComponentBeginOverlap(Capsule)
  (params (OverlappedComponent :type Primitive%20Component%20Object%20Reference) (OtherActor :type Actor%20Object%20Reference) (OtherComp :type Primitive%20Component%20Object%20Reference) (OtherBodyIndex :type Integer) (bFromSweep :type Boolean) (SweepResult :type Hit%20Result%20Structure%20%28by%20ref%29))
  ;[1 1 1] Damage Player
  (bind _asbp_player (Utilities|Casting|CastToBP_Player OtherActor))
  (Game|Damage|ApplyDamage _asbp_player 3e+01 0 0))

(fn ConstructionScript)